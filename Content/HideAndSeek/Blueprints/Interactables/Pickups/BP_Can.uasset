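; A collectible can pickup for the hide-and-seek mode that spins idly until a player-controlled pawn overlaps its collider.
; On pickup it disables collision and reports itself to BP_HideAndSeekGameMode via PickUpCan.
; A PickUp timeline then replaces the idle spin, driving extra rotation, vertical offset and material opacity on the mesh.
; A timer destroys the actor after DespawnDelay.
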(event OnComponentBeginOverlap(Collider)
  (params (OverlappedComponent :type Primitive%20Component%20Object%20Reference) (OtherActor :type Actor%20Object%20Reference) (OtherComp :type Primitive%20Component%20Object%20Reference) (OtherBodyIndex :type Integer) (bFromSweep :type Boolean) (SweepResult :type Hit%20Result%20Structure%20%28by%20ref%29))
  (bind _canmesh (Variables|Default|GetCanMesh))
  (bind _aspawn (Utilities|Casting|CastToPawn OtherActor))
  (if (Pawn|IsPlayerControlled _aspawn)
    (Collision|SetCollisionEnabled (Variables|Default|GetCollider) "NoCollision")
    (bind _asbp_hide_and_seek_game_mode (Utilities|Casting|CastToBP_HideAndSeekGameMode (Game|GetGameMode)))
    (Default|PickUpCan _asbp_hide_and_seek_game_mode self)
    (Utilities|FlowControl|Sequence
      (:then_0
        (bind _additionalrotation (Timeline|IdleSpin Stop)
          (:Update
            (Transformation|SetWorldRotation (Variables|Default|GetCanMesh) (Math|Rotator|MakeRotator (.roll (Variables|Default|GetStartCoinRotation)) (.pitch (Variables|Default|GetStartCoinRotation)) (+ (.yaw (Variables|Default|GetStartCoinRotation)) _additionalrotation)) false false))))
      (:then_1
        (Variables|Default|SetStartCoinRotation (Transformation|GetWorldRotation _canmesh))
        (Variables|Default|SetStartCoinLocation (Variables|/Script/Engine.SceneComponent|GetRelativeLocation _canmesh))
        (bind (_direction _additionalrotation_2 _additionalzoffset _opacity) (Timeline|PickUp Play)
          (:Update
            (Transformation|SetWorldRotation (Variables|Default|GetCanMesh) (Math|Rotator|MakeRotator (.roll (Variables|Default|GetStartCoinRotation)) (.pitch (Variables|Default|GetStartCoinRotation)) (+ (.yaw (Variables|Default|GetStartCoinRotation)) _additionalrotation_2)) false false)
            (Transformation|SetRelativeLocation (Variables|Default|GetCanMesh) (Math|Vector|MakeVector (.x (Variables|Default|GetStartCoinLocation)) (.y (Variables|Default|GetStartCoinLocation)) (+ (.z (Variables|Default|GetStartCoinLocation)) _additionalzoffset)) false false)
            (Rendering|Material|SetScalarParameterValueonMaterials (Variables|Default|GetCanMesh) "Opacity" _opacity))))
      (:then_2
        (Utilities|Time|SetTimerbyEvent (delegate Custom|OnDespawnDelayOver) (Variables|Default|GetDespawnDelay))))))

(event Custom|OnDespawnDelayOver
  (bind _startcoinrotation (Variables|Default|GetStartCoinRotation))
  (bind _startcoinlocation (Variables|Default|GetStartCoinLocation))
  (Utilities|FlowControl|Sequence
    (:then_0
      (bind (_direction _additionalrotation _additionalzoffset _opacity) (Timeline|PickUp Stop)
        (:Update
          (Transformation|SetWorldRotation (Variables|Default|GetCanMesh) (Math|Rotator|MakeRotator (.roll _startcoinrotation) (.pitch _startcoinrotation) (+ (.yaw _startcoinrotation) _additionalrotation)) false false)
          (Transformation|SetRelativeLocation (Variables|Default|GetCanMesh) (Math|Vector|MakeVector (.x _startcoinlocation) (.y _startcoinlocation) (+ (.z _startcoinlocation) _additionalzoffset)) false false)
          (Rendering|Material|SetScalarParameterValueonMaterials (Variables|Default|GetCanMesh) "Opacity" _opacity))))
    (:then_1
      (Actor|DestroyActor))))

(event EventBeginPlay
  (Variables|Default|SetStartCoinRotation (Transformation|GetWorldRotation (Variables|Default|GetCanMesh)))
  (bind _additionalrotation (Timeline|IdleSpin Play)
    (:Update
      (Transformation|SetWorldRotation (Variables|Default|GetCanMesh) (Math|Rotator|MakeRotator (.roll (Variables|Default|GetStartCoinRotation)) (.pitch (Variables|Default|GetStartCoinRotation)) (+ (.yaw (Variables|Default|GetStartCoinRotation)) _additionalrotation)) false false))))

(fn ConstructionScript)