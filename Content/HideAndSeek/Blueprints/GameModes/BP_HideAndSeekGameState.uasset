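; Game state for the Hide and Seek mode that tracks the can score and the current floor height.
; PickUpCan adds one can, and LoseCans subtracts a requested amount, clamped at zero, and returns how many were actually lost.
; SetFloorHeight stores the height and pushes it to the MPC_Occluder material parameter collection, so materials using that collection receive the value.
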(event EventBeginPlay)

(event EventTick
  (params (DeltaSeconds :type Float%20%28single-precision%29)))

(fn ConstructionScript)

(fn PickUpCan
  (Variables|Default|SetCanScore (+ (Variables|Default|GetCanScore) 1)))

(fn GetCanScore
  (return (Variables|Default|GetCanScore)))

(fn LoseCans
  (params (CansLost :type Integer))
  (if (> (- (Variables|Default|GetCanScore) CansLost) 0)
    (Variables|Default|SetCanScore (- (Variables|Default|GetCanScore) CansLost))
    (return CansLost)
    (else
      (LocalVariables|SetActualScoreLoss (Variables|Default|GetCanScore))
      (Variables|Default|SetCanScore 0)
      (return (LocalVariables|GetActualScoreLoss)))))

(fn SetFloorHeight
  (params (FloorHeight :type Float%20%28double-precision%29))
  (bind _output_get (Variables|Default|SetFloorHeight FloorHeight))
  (Rendering|Material|SetScalarParameterValue "/Game/HideAndSeek/Materials/MPC_Occluder.MPC_Occluder" "FloorHeight" _output_get :!class /Script/Engine.KismetMaterialLibrary))

(fn GetFloorHeight
  (return (Variables|Default|GetFloorHeight)))