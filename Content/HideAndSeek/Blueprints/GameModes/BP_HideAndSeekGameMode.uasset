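; Game mode for a hide-and-seek game that runs NPC and can spawning and the HUD.
; Spawn points and can spawners register themselves; after a short delay, random points spawn NPCs with patrol routes and random spawners fill cans up to a cap.
; Pickups update the game state and refill cans, excluding the just-used spawner.
; It also forwards can losses to the game state and NPC dialogue lines to the HUD.
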(event EventBeginPlay
  (Utilities|FlowControl|Delay 1.0)
  (CallFunction|SpawnEnemies)
  (CallFunction|PopulateCans)
  (CallFunction|CreateHUD)
  (bind _asbp_hide_and_seek_game_state (Utilities|Casting|CastToBP_HideAndSeekGameState (Game|GetGameState)))
  (Variables|Default|SetState _asbp_hide_and_seek_game_state))

(event EventTick
  (params (DeltaSeconds :type Float%20%28single-precision%29)))

(fn ConstructionScript)

(fn RegisterNPCSpawnPoint
  (params (NewSpawnPoint :type BP%20NPC%20Spawn%20Point%20Object%20Reference))
  (Utilities|Array|Add (Variables|Default|GetSpawnPoints) NewSpawnPoint))

(fn PickUpCan
  (params (PickedUpCoin :type BP%20Can%20Object%20Reference))
  (bind _asbp_hide_and_seek_game_state (Utilities|Casting|CastToBP_HideAndSeekGameState (Game|GetGameState)))
  (Default|PickUpCan _asbp_hide_and_seek_game_state)
  (bind _keys (Utilities|Map|Keys (Variables|Default|GetActiveCans)))
  (bind _array_element (Utilities|Array|ForEachLoopwithBreak _keys :!label _label)
    (:LoopBody
      (if (== (.Value (Utilities|Map|Find (Variables|Default|GetActiveCans) _array_element)) PickedUpCoin)
        (Variables|Default|SetJustUsedSpawner _array_element)
        (Utilities|Map|Remove (Variables|Default|GetActiveCans) _array_element)
        (goto _label Break)))
    (:Completed
      (CallFunction|PopulateCans))))

(fn RegisterCanSpawner
  (params (CoinSpawner :type BP%20Can%20Spawner%20Object%20Reference))
  (Utilities|Array|AddUnique (Variables|Default|GetCanSpawners) CoinSpawner))

(fn SpawnEnemies
  (for _array_element (Variables|Default|GetSpawnPoints)
    (Utilities|Array|Add (LocalVariables|GetUnusedSpawnPoints) _array_element))
  (Utilities|FlowControl|ForLoopwithBreak 1 (Variables|Default|GetMaxActiveEnemies) :!label _label
    (:LoopBody
      (if (> (Utilities|Array|Length (LocalVariables|GetUnusedSpawnPoints)) 0)
        (bind _output_get (LocalVariables|SetActiveSpawnPoint (.OutItem (Utilities|Array|Random (LocalVariables|GetUnusedSpawnPoints)))))
        (bind (_npc _spawnsuccessful) (Default|SpawnNPC _output_get))
        (if _spawnsuccessful
          (bind _asbp_npc_controller (Utilities|Casting|CastToBP_NPC_Controller (Pawn|GetController _npc)))
          (Default|SetPatrolRoute _asbp_npc_controller (Variables|/Game/HideAndSeek/Blueprints/Placeables/BP_NPCSpawnPoint.BP_NPCSpawnPoint_C|GetPatrolRoute _output_get))
          (Utilities|Array|RemoveItem (LocalVariables|GetUnusedSpawnPoints) _output_get))
        (else
          (goto _label Break))))))

(fn PopulateCans
  (bind _keys (Utilities|Map|Keys (Variables|Default|GetActiveCans)))
  (if (< (Utilities|Array|Length _keys) (Variables|Default|GetMaxActiveCans))
    (for _array_element (Variables|Default|GetCanSpawners)
      (if (not (Utilities|Array|ContainsItem _keys _array_element))
        (Utilities|Array|Add (LocalVariables|GetUnusedCanSpawners) _array_element)))
    (Utilities|Array|RemoveItem (LocalVariables|GetUnusedCanSpawners) (Variables|Default|GetJustUsedSpawner))
    (Utilities|FlowControl|ForLoopwithBreak 1 (- (Variables|Default|GetMaxActiveCans) (Utilities|Array|Length _keys)) :!label _label
      (:LoopBody
        (if (> (Utilities|Array|Length (LocalVariables|GetUnusedCanSpawners)) 0)
          (bind _output_get (LocalVariables|SetActiveCanSpawner (.OutItem (Utilities|Array|Random (LocalVariables|GetUnusedCanSpawners)))))
          (bind (_can _spawnsuccessful) (Default|SpawnCan _output_get))
          (if _spawnsuccessful
            (Utilities|Map|Add (Variables|Default|GetActiveCans) (LocalVariables|GetActiveCanSpawner) _can)
            (Utilities|Array|RemoveItem (LocalVariables|GetUnusedCanSpawners) (LocalVariables|GetActiveCanSpawner)))
          (else
            (goto _label Break)))))))

(fn CreateHUD
  (bind _returnvalue (UserInterface|CreateWidget "/Game/HideAndSeek/Blueprints/UI/WBP_HUD.WBP_HUD_C" (Game|GetPlayerController 0)))
  (bind _output_get (Variables|Default|SetHUD _returnvalue))
  (UserInterface|Viewport|AddtoViewport _output_get 0))

(fn LoseCans
  (params (CoinsLost :type Integer))
  (bind _actualcanslost (Default|LoseCans (Variables|Default|GetState) CoinsLost))
  (return _actualcanslost))

(fn QueueNPCLine
  (params (NPC :type BP%20NPC%20Object%20Reference) (Line :type String) (Duration :type Float%20%28double-precision%29) (Urgent :type Boolean))
  (Default|QueueDialogueLine (Variables|Default|GetHUD) NPC Line Duration Urgent))