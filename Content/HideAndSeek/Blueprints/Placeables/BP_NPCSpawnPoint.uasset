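; BP_NPCSpawnPoint is a placeable spawn point for NPCs in the Hide and Seek mode.
; Half a second after BeginPlay it registers itself with BP_HideAndSeekGameMode.
; SpawnNPC spawns the configured NPCType at the point's transform, adjusting for collisions but always spawning, stores the result and reports success, printing an error on failure.
; GetNPC returns the stored NPC.
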(event EventBeginPlay
  (Utilities|FlowControl|Delay 0.5)
  (bind _asbp_hide_and_seek_game_mode (Utilities|Casting|CastToBP_HideAndSeekGameMode (Game|GetGameMode)))
  (Default|RegisterNPCSpawnPoint _asbp_hide_and_seek_game_mode self))

(event Collision|EventActorBeginOverlap
  (params (OtherActor :type Actor%20Object%20Reference)))

(event EventTick
  (params (DeltaSeconds :type Float%20%28single-precision%29)))

(fn ConstructionScript)

(fn SpawnNPC
  (bind _returnvalue (Game|SpawnActorfromClass (Variables|Default|GetNPCType) (Transformation|GetActorTransform) "AdjustIfPossibleButAlwaysSpawn" "MultiplyWithRoot" 0 0))
  (if (Utilities|IsValid _returnvalue)
    (bind _output_get (Variables|Default|SetNPC _returnvalue))
    (return _output_get true)
    (else
      (Development|PrintString "[ERROR][Spawn Point] NPC spawning unsuccessful." false true "(R=1.000000,G=0.017051,B=0.000000,A=1.000000)")
      (return 0 false))))

(fn GetNPC
  (return (Variables|Default|GetNPC)))