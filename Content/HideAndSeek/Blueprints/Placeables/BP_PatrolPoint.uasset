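; BP_PatrolPoint is a placeable patrol point for hide-and-seek NPCs, storing an idle time that other code reads through GetIdleTime.
; SetActive shows the point's state by switching the preview cylinder's material between red for active and blue for inactive.
; The trigger sphere's overlap handler casts to BP_NPC and its controller but takes no further action.
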(event OnComponentBeginOverlap(TriggerSphere)
  (params (OverlappedComponent :type Primitive%20Component%20Object%20Reference) (OtherActor :type Actor%20Object%20Reference) (OtherComp :type Primitive%20Component%20Object%20Reference) (OtherBodyIndex :type Integer) (bFromSweep :type Boolean) (SweepResult :type Hit%20Result%20Structure%20%28by%20ref%29))
  (bind _asbp_npc (Utilities|Casting|CastToBP_NPC OtherActor))
  (Utilities|Casting|CastToBP_NPC_Controller (Pawn|GetController _asbp_npc)))

(event EventBeginPlay)

(event Collision|EventActorBeginOverlap
  (params (OtherActor :type Actor%20Object%20Reference)))

(event EventTick
  (params (DeltaSeconds :type Float%20%28single-precision%29)))

(fn ConstructionScript)

(fn SetActive
  (params (IsActive :type Boolean))
  (bind _previewcylinder (Variables|Default|GetPreviewCylinder))
  (if IsActive
    (Rendering|Material|SetMaterial _previewcylinder 0 "/Game/HideAndSeek/Materials/Solids/MI_SolidMasked_Red.MI_SolidMasked_Red")
    (else
      (Rendering|Material|SetMaterial _previewcylinder 0 "/Game/HideAndSeek/Materials/Solids/MI_SolidMasked_Blue.MI_SolidMasked_Blue"))))

(fn GetIdleTime
  (return (Variables|Default|GetIdleTimeAtPoint)))