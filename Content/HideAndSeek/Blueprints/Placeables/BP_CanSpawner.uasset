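; BP_CanSpawner is a placeable spawn point for the BP_Can actor in the Hide and Seek mode.
; Shortly after BeginPlay, a brief timer delays registering it with BP_HideAndSeekGameMode.
; Its SpawnCan function spawns a BP_Can at the spawner's transform and returns the can with a success flag, printing an error on failure.
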(event Custom|OnGameModeReady
  (bind _asbp_hide_and_seek_game_mode (Utilities|Casting|CastToBP_HideAndSeekGameMode (Game|GetGameMode)))
  (Default|RegisterCanSpawner _asbp_hide_and_seek_game_mode self))

(event EventBeginPlay
  (Utilities|Time|SetTimerbyEvent (delegate Custom|OnGameModeReady) 0.3))

(fn ConstructionScript)

(fn SpawnCan
  (bind _returnvalue (Game|SpawnActorfromClass "/Game/HideAndSeek/Blueprints/Interactables/Pickups/BP_Can.BP_Can_C" (Transformation|GetActorTransform) "Undefined" "MultiplyWithRoot" 0 0))
  (if (Utilities|IsValid _returnvalue)
    (return _returnvalue true)
    (else
      (Development|PrintString "[ERROR][Can Spawner] Can spawning unsuccessful." false true "(R=1.000000,G=0.017051,B=0.000000,A=1.000000)")
      (return 0 false))))