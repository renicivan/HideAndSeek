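; Player character for the HideAndSeek game that feeds occlusion material data and reacts to hits.
; It writes its spawn location on BeginPlay, then player and camera locations every Tick, into the MPC_Occluder parameter collection.
; GetHit has the game mode deduct cans, launches the character away from the hit origin with an upward bias, and spawns Niagara particles matching the cans lost.
; A floor-number debug print is left unconnected.
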(event EventTick
  (params (DeltaSeconds :type Float%20%28single-precision%29))
  (Rendering|Material|SetVectorParameterValue "/Game/HideAndSeek/Materials/MPC_Occluder.MPC_Occluder" "CurrentPlayerLocation" (Math|Conversions|ToLinearColor(Vector) (Transformation|GetActorLocation)) :!class /Script/Engine.KismetMaterialLibrary)
  (Rendering|Material|SetVectorParameterValue "/Game/HideAndSeek/Materials/MPC_Occluder.MPC_Occluder" "CurrentCameraLocation" (Math|Conversions|ToLinearColor(Vector) (Transformation|GetWorldLocation (Variables|Camera|GetCamera))) :!class /Script/Engine.KismetMaterialLibrary)
  (bind _returnvalue (Rendering|Material|GetVectorParameterValue "/Game/HideAndSeek/Materials/MPC_Occluder.MPC_Occluder" "SpawnLocation" :!class /Script/Engine.KismetMaterialLibrary))
  (bind _returnvalue_2 (Rendering|Material|GetVectorParameterValue "/Game/HideAndSeek/Materials/MPC_Occluder.MPC_Occluder" "CurrentPlayerLocation" :!class /Script/Engine.KismetMaterialLibrary))
  (bind _returnvalue_3 (Rendering|Material|GetScalarParameterValue "/Game/HideAndSeek/Materials/MPC_Occluder.MPC_Occluder" "FloorHeight" :!class /Script/Engine.KismetMaterialLibrary)))

(event EventBeginPlay
  (Rendering|Material|SetVectorParameterValue "/Game/HideAndSeek/Materials/MPC_Occluder.MPC_Occluder" "SpawnLocation" (Math|Conversions|ToLinearColor(Vector) (Transformation|GetActorLocation)) :!class /Script/Engine.KismetMaterialLibrary))

(fn ConstructionScript)

(fn GetHit
  (params (CoinDamage :type Integer) (HitOrigin :type Vector))
  (bind _niagara (Variables|Default|GetNiagara))
  (bind _asbp_hide_and_seek_game_mode (Utilities|Casting|CastToBP_HideAndSeekGameMode (Game|GetGameMode)))
  (bind _actualcoinslost (Default|LoseCans _asbp_hide_and_seek_game_mode CoinDamage))
  (Character|LaunchCharacter (* (Math|Vector|Normalize (- (+ (Transformation|GetActorLocation) "0.000000,0.000000,50.000000") HitOrigin)) 5e+02) false false)
  (Class|NiagaraComponent|SetVariableInt _niagara "User.SpawnCount" _actualcoinslost)
  (Components|Activation|Activate _niagara false))