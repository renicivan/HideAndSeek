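; Base NPC character for the hide-and-seek game, with AI perception, switchable movement types and spoken lines.
; On BeginPlay it spawns its controller and sets an initial movement type, which looks up max walk speed from a map.
; Perception updates go to TargetTrackerComponent for evaluation.
; Getters supply display name, image, colors and random target sighted, acquired or lost lines, while SaySomething queues lines through the game mode.
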(event OnTargetPerceptionUpdated(AIPerception)
  (params (Actor :type Actor%20Object%20Reference) (Stimulus :type AI%20Stimulus%20Structure))
  (Default|EvaluateStimulus (Variables|Default|GetTargetTrackerComponent) Actor Stimulus))

(event EventBeginPlay
  (Pawn|SpawnDefaultController)
  (CallFunction|SetMovementType "NewEnumerator0"))

(fn ConstructionScript)

(fn SetMovementType
  (params (NewMovementType :type EMovementType%20Enum :default "NewEnumerator0"))
  (bind _output_get (Variables|Default|SetCurrentMovementType NewMovementType))
  (Variables|/Script/Engine.CharacterMovementComponent|SetMaxWalkSpeed (Variables|Character|GetCharacterMovement) (.Value (Utilities|Map|Find (Variables|Default|GetMovementTypes) _output_get))))

(fn GetCapsuleHalfHeight
  (return (Variables|/Script/Engine.CapsuleComponent|GetCapsuleHalfHeight (Variables|Collision|GetCapsuleComponent))))

(fn GetName
  (return (Variables|Default|GetName)))

(fn GetBackgroundColor
  (return (Variables|Default|GetBackgroundColor)))

(fn GetImage
  (return (Variables|Default|GetImage)))

(fn SaySomething
  (params (Line :type String) (Duration :type Float%20%28double-precision%29) (Urgent :type Boolean))
  (bind _asbp_hide_and_seek_game_mode (Utilities|Casting|CastToBP_HideAndSeekGameMode (Game|GetGameMode)))
  (Default|QueueNPCLine _asbp_hide_and_seek_game_mode self Line Duration Urgent))

(fn GetHeaderColor
  (return (Variables|Default|GetHeaderColor)))

(fn GetTextColor
  (return (Variables|Default|GetTextColor)))

(fn GetTargetAcquiredLine
  (return (.OutItem (Utilities|Array|Random (Variables|Default|GetTargetAcquiredLines)))))

(fn GetTargetLostLine
  (return (.OutItem (Utilities|Array|Random (Variables|Default|GetTargetLostLines)))))

(fn GetTargetSightedLine
  (return (.OutItem (Utilities|Array|Random (Variables|Default|GetTargetSightedLines)))))