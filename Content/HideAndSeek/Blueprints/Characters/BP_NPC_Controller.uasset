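; BP_NPC_Controller is the AI controller for hide-and-seek NPCs, starting the BT_BasicNPC behavior tree on BeginPlay.
; It writes the patrol route to the blackboard and forwards movement type and speech lines to the possessed BP_NPC.
; ActivateAttack sphere-traces forward from the pawn and calls GetHit with coin damage on a hit BP_TopDownCharacter.
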(event EventBeginPlay
  (AI|RunBehaviorTree "/Game/HideAndSeek/AI/BehaviorTrees/BT_BasicNPC.BT_BasicNPC"))

(fn ConstructionScript)

(fn SetPatrolRoute
  (params (PatrolRoute :type BP%20Patrol%20Route%20Object%20Reference))
  (AI|Components|Blackboard|SetValueasObject (AI|GetBlackboard 0) (Utilities|Name|MakeLiteralName "PatrolRoute") PatrolRoute))

(fn SetMovementType
  (params (NewMovementType :type EMovementType%20Enum :default "NewEnumerator0"))
  (bind _asbp_npc (Utilities|Casting|CastToBP_NPC (Pawn|GetControlledPawn)))
  (Default|SetMovementType _asbp_npc NewMovementType))

(fn ActivateAttack
  (bind _returnvalue (Pawn|GetControlledPawn))
  (bind _returnvalue_2 (Transformation|GetActorLocation _returnvalue))
  (bind (_outhit _returnvalue_3) (Collision|SphereTraceForObjects _returnvalue_2 (+ _returnvalue_2 (* (Math|Vector|Normalize (Math|Vector|GetForwardVector (Transformation|GetActorRotation _returnvalue))) 5e+02)) 3e+01 (Utilities|Array|MakeArray "ObjectTypeQuery3") false (Utilities|Array|MakeArray _returnvalue) "None"))
  (if _returnvalue_3
    (bind _asbp_top_down_character (Utilities|Casting|CastToBP_TopDownCharacter (.HitActor (Collision|BreakHitResult _outhit))))
    (Default|GetHit _asbp_top_down_character 2 (.ImpactPoint (Collision|BreakHitResult _outhit)))))

(fn SaySomething
  (params (Line :type String) (Duration :type Float%20%28double-precision%29))
  (bind _asbp_npc (Utilities|Casting|CastToBP_NPC (Pawn|GetControlledPawn)))
  (Default|SaySomething _asbp_npc Line Duration false))